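; Forest is an actor Blueprint that builds a grid of tree meshes when placed or edited.
; Its construction script, when TreeMesh is valid, loops over NumX by NumY and adds a static mesh component per cell.
; Cell spacing comes from the mesh's bounding box width and depth, so trees sit edge to edge on a flat plane.
; The event graph holds no active logic.
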(event EventBeginPlay)

(event Collision|EventActorBeginOverlap
  (params (OtherActor :type Actor%20Object%20Reference)))

(event EventTick
  (params (DeltaSeconds :type Float%20%28single-precision%29)))

(fn ConstructionScript
  (bind _treemesh (Variables|Rendering|GetTreeMesh))
  (bind _returnvalue (StaticMesh|GetBoundingBox _treemesh))
  (bind (_min _max) (Utilities|Struct|BreakBox _returnvalue))
  (bind (_x _y) (Math|Vector|BreakVector _min))
  (bind (_x_2 _y_2) (Math|Vector|BreakVector _max))
  (Utilities|IsValid (Variables|Rendering|GetTreeMesh)
    (:Is%20Valid
      (for _index (range 0 (- (Variables|Rendering|GetNumX) 1))
        (for _index_2 (range 0 (- (Variables|Rendering|GetNumY) 1))
          (bind _returnvalue_2 (AddComponent|AddStaticMeshComponent false (Math|Transform|MakeTransform (Math|Vector|MakeVector (* _index (- _x_2 _x)) (* _index_2 (- _y_2 _y)) 0.0))))
          (Components|StaticMesh|SetStaticMesh _returnvalue_2 (Variables|Rendering|GetTreeMesh)))))))