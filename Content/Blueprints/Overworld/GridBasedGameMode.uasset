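; Overworld game mode for grid-based movement that handles screen fades, wild Pokémon encounters and repel steps.
; Encounter checks pass the character's location-based encounter type through RandomEncounterSubsystem, then start a single wild battle, guarded by an InEncounter flag.
; Repel steps count down except on ice; expiry shows a message, offering another from the bag if available, otherwise the encounter check runs.
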(event EventCheckRepelSteps
  (params (Character :type Character%20Object%20Reference))
  (if (Math|Boolean|NORBoolean (Class|TerrainTagUtilities|HasTerrainTag "(TagName=\"Terrain.Ice\")" Character) (not (Class|TrainerHelpers|IsRepelActive)))
    (Class|TrainerHelpers|DecrementRepelSteps)
    (if (not (Class|TrainerHelpers|IsRepelActive))
      (if (Class|Bag|HasItemwithTag (Class|TrainerHelpers|GetBag) "Repel")
        (|DisplayMessagewithChoices "The repellent's effect wore off! Would you like to use another one?" "Yes" "No"
          (:Choice0_Output
            (bind (_screen _item) (|ChooseItemfromBag (EventDispatchers|CreateEvent :!event IsRepel))
              (:OnSelected
                (|UseItemDirect (.AsBag%20Screen (Utilities|Casting|CastToBagScreen _screen)) (Utilities|Struct|BreakItem _item))))))
        (else
          (|DisplayMessage "The repellent's effect wore off!")))
      (else
        (CallFunction|CheckforEncounter Character (Class|TrainerHelpers|IsRepelActive) :!label _label)))
    (else
      (goto _label))))

(event EventScreenFadein
  (CameraFades|StartCameraFade :self (Game|GetPlayerCameraManager 0) :FromAlpha 1.0 :Duration 0.15 :bHoldWhenFinished true)
  (Utilities|FlowControl|Delay 0.2)
  (Class|GridBasedGameModeBase|ScreenTransitionFinished))

(event EventScreenFadeOut
  (CameraFades|StartCameraFade :self (Game|GetPlayerCameraManager 0) :ToAlpha 1.0 :Duration 0.15 :bHoldWhenFinished true)
  (Utilities|FlowControl|Delay 0.2)
  (Class|GridBasedGameModeBase|ScreenTransitionFinished))

(event EventCheckforEncounter
  (params (Character :type Character%20Object%20Reference) (IsRepelActive :type Boolean))
  (bind _returnvalue (Subsystems|GetRandomEncounterSubsystem))
  (if (not (Variables|Default|GetInEncounter))
    (if (> (Class|Trainer|GetAblePokemonCount (Class|TrainerHelpers|GetPlayerCharacter)) 0)
      (bind _encounterpossible (CallFunction|EncounterPossibleHere Character))
      (if _encounterpossible
        (bind _encountertype (CallFunction|GetEncounterType Character))
        (if (GameplayTags|IsGameplayTagValid _encountertype)
          (bind _returnvalue_2 (Class|RandomEncounterSubsystem|CheckEncounterTriggered _returnvalue Character _encountertype IsRepelActive true))
          (if _returnvalue_2
            (bind _encounter (Class|RandomEncounterSubsystem|RequestEncounterforType _returnvalue _encountertype 1)
              (:True
                (bind _returnvalue_3 (Class|RandomEncounterSubsystem|AllowEncounter _returnvalue _encounter IsRepelActive))
                (if _returnvalue_3
                  (Variables|Default|SetInEncounter true)
                  (|InitiateBattle (Class|BattleTransitionHelpers|MakeSingleWildBattle (Class|SpeciesHelper|ConvertNametoSpeciesHandle (.Species (Utilities|Struct|BreakRetrievedEncounter _encounter))) (.Level (Utilities|Struct|BreakRetrievedEncounter _encounter)) false) (Variables|Default|GetEncounterTransition)
                    (:AfterBattle
                      (Variables|Default|SetInEncounter false))))))))))))

(event EventBeginPlay
  (Class|PlayerCameraManager|SetManualCameraFade :self (Game|GetPlayerCameraManager 0) :InFadeAmount 1.0)
  (Utilities|FlowControl|Delay 0.2)
  (CameraFades|StartCameraFade :self (Game|GetPlayerCameraManager 0) :FromAlpha 1.0 :Duration 0.15 :bHoldWhenFinished true)
  (Utilities|FlowControl|Delay 0.2)
  (Class|GridBasedGameModeBase|ScreenTransitionFinished))

(fn ConstructionScript)

(fn IsRepel
  (params (Item :type Item%20Structure%20%28by%20ref%29))
  (return (Utilities|Array|ContainsItem (Utilities|Struct|BreakItem Item) "Repels")))