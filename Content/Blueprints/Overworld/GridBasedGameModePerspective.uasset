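; Overworld game mode that handles screen fade transitions and swaps lighting profiles.
; Camera fades in or out through the player camera manager, then fires OnScreenTransitionFinished after a shared short delay; BeginPlay starts on black and fades in.
; SetLightingProfile does a blocking unload of the current lighting level and streams in the new one, with its same-profile comparison left unconnected.
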(event EventSetLightingProfile
  (params (NewLightingProfile :type Soft%20World%20Reference%20Structure))
  (Class|GameplayStatics|UnloadStreamLevelbySoftObjectPtr (Variables|Default|GetCurrentLightingProfile) true)
  (bind _output_get (Variables|Default|SetCurrentLightingProfile (Utilities|Struct|BreakSoftWorldReference NewLightingProfile)))
  (Class|GameplayStatics|LoadStreamLevelbySoftObjectPtr _output_get true true))

(event EventScreenFadein
  (CameraFades|StartCameraFade :self (Game|GetPlayerCameraManager 0) :FromAlpha 1.0 :Duration 0.15 :bHoldWhenFinished true)
  (Utilities|FlowControl|Delay 0.2)
  (Default|CallOnScreenTransitionFinished))

(event EventScreenFadeOut
  (CameraFades|StartCameraFade :self (Game|GetPlayerCameraManager 0) :ToAlpha 1.0 :Duration 0.15 :bHoldWhenFinished true)
  (Utilities|FlowControl|Delay 0.2)
  (Default|CallOnScreenTransitionFinished))

(event EventBeginPlay
  (Class|PlayerCameraManager|SetManualCameraFade :self (Game|GetPlayerCameraManager 0) :InFadeAmount 1.0)
  (Utilities|FlowControl|Delay 0.2)
  (CameraFades|StartCameraFade :self (Game|GetPlayerCameraManager 0) :FromAlpha 1.0 :Duration 0.15 :bHoldWhenFinished true)
  (Utilities|FlowControl|Delay 0.2)
  (Default|CallOnScreenTransitionFinished))

(fn ConstructionScript)