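; Test actor that exercises gameplay effects on a battler's stats through its BattlerAbility ability system component.
; BeginPlay applies a test stat effect, then a stage-change effect whose attack magnitude is set by caller through the Battle.Stats.Stages tag, then a stat-stages effect.
; Tick prints every attribute value as text for inspection.
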(event EventBeginPlay
  (bind _battlerability (Variables|Default|GetBattlerAbility))
  (GameplayEffects|ApplyGameplayEffectToSelf (Variables|Default|GetBattlerAbility) "/Game/Blueprints/Testing/SetTestStats.SetTestStats_C" 0.0 (GameplayEffects|MakeEffectContext (Variables|Default|GetBattlerAbility)))
  (bind _returnvalue (Ability|GameplayEffect|AssignTagSetbyCallerMagnitude (GameplayEffects|MakeOutgoingSpec _battlerability "/Game/Blueprints/Battle/GameplayAbilities/Effects/Active/ChangeAttackStages.ChangeAttackStages_C" 0.0 (GameplayEffects|MakeEffectContext _battlerability)) "(TagName=\"Battle.Stats.Stages\")" 2.0))
  (GameplayEffects|ApplyGameplayEffectSpecToSelf (Variables|Default|GetBattlerAbility) _returnvalue)
  (GameplayEffects|ApplyGameplayEffectToSelf (Variables|Default|GetBattlerAbility) "/Game/Blueprints/Battle/GameplayAbilities/Effects/Effect_StatStages.Effect_StatStages_C" 0.0 (GameplayEffects|MakeEffectContext (Variables|Default|GetBattlerAbility))))

(event EventTick
  (params (DeltaSeconds :type Float%20%28single-precision%29))
  (for _array_element (Class|AbilitySystemComponent|GetAllAttributes (Variables|Default|GetBattlerAbility))
    (Development|PrintText (Utilities|Text|ToText(Float) (.ReturnValue (Ability|Attribute|GetFloatAttribute self _array_element)) "HalfToEven"))))

(fn ConstructionScript)