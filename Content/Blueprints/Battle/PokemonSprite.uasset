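; PokemonSprite is a battle actor that displays a Pokémon as a Paper2D flipbook.
; A CameraFacingRotator component is given the flipbook as its rotated component, both in the construction script and on BeginPlay, apparently to billboard the sprite toward the camera.
; SetBattleSprite swaps the displayed flipbook, and Faint hides the actor in game.
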(event EventBeginPlay
  (Variables|/Script/GridBased2D.CameraFacingRotatorComponent|SetRotatedComponent (Variables|Default|GetCameraFacingRotator) (Variables|Default|GetPaperFlipbook)))

(event EventSetBattleSprite
  (params (Flipbook :type Paper%20Flipbook%20Object%20Reference))
  (Sprite|SetFlipbook (Variables|Default|GetPaperFlipbook) Flipbook))

(event EventFaint
  (Rendering|SetActorHiddenInGame true))

(fn ConstructionScript
  (Variables|/Script/GridBased2D.CameraFacingRotatorComponent|SetRotatedComponent (Variables|Default|GetCameraFacingRotator) (Variables|Default|GetPaperFlipbook)))