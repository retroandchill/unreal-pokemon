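; Battle Poke Ball actor that plays the throw animation sending a Battler's sprite into battle, with a camera-facing flipbook.
; ThrowPokeBall plays a sound and runs a timeline that moves the ball toward a point above the Battler, adding a height offset.
; On arrival it hides the ball, shows the Battler's sprite, lerps the Battler from the ball's position to its original location, then destroys itself.
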(event EventThrowPokeBall
  (params (Destination :type Vector :default "0, 0, 0"))
  (Variables|Default|SetDestination (|GetDestination))
  (Variables|Default|SetStartingLocation (Transformation|GetActorLocation))
  (Audio|PlaySound2D "/Game/Audio/SE/Battle/Throw.Throw" 1.0 1.0 0.0 0 0)
  (bind (_direction _distance _z_offset) (Timeline|ThrowAnimation Play)
    (:Update
      (Transformation|SetActorLocation (|GuideToDestination _distance _z_offset) false false))
    (:Finished
      (bind _asactor (Utilities|Casting|CastToActor (Variables|Context|GetBattler)))
      (Variables|Default|SetOriginalLocation (Transformation|GetActorLocation _asactor))
      (Transformation|SetActorLocation _asactor (Transformation|GetActorLocation _asactor) false false)
      (Class|Battler|ShowSprite (Variables|Context|GetBattler) "0, 0, 0")
      (Development|SetHiddeninGame (Variables|Default|GetPaperFlipbook) true false)
      (bind _distance_2 (Timeline|DropDown Play)
        (:Update
          (Transformation|SetActorLocation _asactor (Math|Vector|Lerp(Vector) (Transformation|GetActorLocation) (Variables|Default|GetOriginalLocation) _distance_2) false false))
        (:Finished
          (Actor|DestroyActor))))))

(fn ConstructionScript
  (Variables|/Script/GridBased2D.CameraFacingRotatorComponent|SetRotatedComponent (Variables|Default|GetCameraFacingRotator) (Variables|Default|GetPaperFlipbook)))

(fn GetDropRate
  (return 1.0))