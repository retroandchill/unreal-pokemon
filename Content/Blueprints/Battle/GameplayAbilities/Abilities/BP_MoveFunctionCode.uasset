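; Gameplay ability base for battle move function codes, handling the on-screen presentation of a move's results.
; Failures show their messages, tag the owner with LastMoveFailed and end the ability.
; Otherwise it shows move messages then calls DealDamage, while DisplayDamage plays each target's HP animation, tracked in an UpdatingBattlers set.
; Macro-style helpers show messages sequentially and poll each tick until that set empties before ending the ability.
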(event Ability|EventActivateAbility)

(event Ability|EventOnEndAbility
  (params (bWasCancelled :type Boolean)))

(event EventProcessMoveFailure
  (params (FailureMessages :type Array%20of%20Texts))
  (Utilities|DisplayEachMessage FailureMessages)
  (Ability|GameplayEffect|AddLooseGameplayTags (Utilities|Struct|BreakGameplayAbilityActorInfo (Ability|GetActorInfo)) (GameplayTags|MakeGameplayTagContainerfromArray (Utilities|Array|MakeArray "(TagName=\"Battle.History.LastMoveFailed\")")))
  (Ability|EndAbility))

(event EventDisplayMessagesandAnimation
  (params (User :type Battler%20Interface%20%28by%20ref%29) (Targets :type Array%20of%20Battler%20Interfaces) (Messages :type Array%20of%20Texts))
  (Utilities|DisplayEachMessage Messages)
  (Class|BattleMoveFunctionCode|DealDamage User Targets))

(event EventDisplayDamage
  (params (User :type Battler%20Interface%20%28by%20ref%29) (Targets :type Array%20of%20Battler%20Interfaces))
  (Utilities|Set|Clear (Variables|Default|GetUpdatingBattlers))
  (for _array_element Targets
    (Utilities|Set|Add (Variables|Default|GetUpdatingBattlers) (Utilities|ToObject(Interface) _array_element))
    (|PlayBattlerHPAnimation _array_element 1.0
      (:OnSelected
        (Utilities|Set|Remove (Variables|Default|GetUpdatingBattlers) (Utilities|ToObject(Interface) _array_element)))))
  (Utilities|WaitUntilConditionIsTrue (Utilities|Set|IsEmpty (Variables|Default|GetUpdatingBattlers)))
  (Ability|EndAbility))