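; Gameplay ability for a battle move in a Pokémon-style game, sequencing the presentation of its outcome.
; Events play each stage (messages, HP animation, effects, fainting), then hand back to damage and effect calls defined outside this graph.
; Critical-hit and effectiveness text comes from target tags and attributes, naming battlers when several are targeted.
; Latent macros pace the flow; failed moves tag the user, and both endings grant faint EXP before ending the ability.
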(event EventProcessMoveFailure
  (params (FailureMessages :type Running%20Message%20Set%20Structure%20%28by%20ref%29))
  (bind _returnvalue (Class|BattleMessageHelper|GetMessages FailureMessages))
  (Utilities|DisplayEachMessage _returnvalue)
  (Ability|GameplayEffect|AddLooseGameplayTags (Utilities|Struct|BreakGameplayAbilityActorInfo (Ability|GetActorInfo)) (GameplayTags|MakeGameplayTagContainerfromArray (Utilities|Array|MakeArray "(TagName=\"Battle.History.LastMoveFailed\")")))
  (Utilities|InvokeEnd))

(event EventDisplayMessagesandAnimation
  (params (User :type Battler%20Interface%20%28by%20ref%29) (Targets :type Array%20of%20Battler%20Interfaces) (Messages :type Running%20Message%20Set%20Structure%20%28by%20ref%29))
  (bind _returnvalue (Class|BattleMessageHelper|GetMessages Messages))
  (Utilities|DisplayEachMessage _returnvalue)
  (Class|BattleMoveFunctionCode|DealDamage User Targets))

(event EventDisplayDamage
  (params (User :type Battler%20Interface%20%28by%20ref%29) (Targets :type Array%20of%20Battler%20Interfaces))
  (Utilities|Set|Clear (Variables|Default|GetUpdatingBattlers))
  (for _array_element Targets
    (Utilities|Set|Add (Variables|Default|GetUpdatingBattlers) (Utilities|ToObject(Interface) _array_element))
    (|PlayBattlerHPAnimation _array_element 1.0
      (:OnSelected
        (Utilities|Set|Remove (Variables|Default|GetUpdatingBattlers) (Utilities|ToObject(Interface) _array_element)))))
  (Utilities|WaitUntilConditionIsTrue (Utilities|Set|IsEmpty (Variables|Default|GetUpdatingBattlers)))
  (Utilities|DisplayDamageResult Targets)
  (Class|BattleMoveFunctionCode|ApplyMoveEffects User Targets))

(event EventFaintCheck
  (params (User :type Battler%20Interface%20%28by%20ref%29) (Targets :type Array%20of%20Battler%20Interfaces) (Messages :type Running%20Message%20Set%20Structure%20%28by%20ref%29))
  (bind _returnvalue (Class|BattleMessageHelper|GetMessages Messages))
  (Utilities|DisplayEachMessage _returnvalue)
  (Utilities|FaintCheckonBattler User)
  (Utilities|FaintCheckonEachTarget Targets)
  (Class|BattleMoveFunctionCode|ApplyAdditionalEffects User Targets))

(event EventDisplayMoveEffectsandEndMove
  (params (User :type Battler%20Interface%20%28by%20ref%29) (Targets :type Array%20of%20Battler%20Interfaces) (Messages :type Running%20Message%20Set%20Structure%20%28by%20ref%29))
  (bind _returnvalue (Class|BattleMessageHelper|GetMessages Messages))
  (Utilities|DisplayEachMessage _returnvalue)
  (Utilities|InvokeEnd))

(fn GetTypeEffectivenessMessages
  (params (Targets :type Array%20of%20Battler%20Interfaces))
  (for _array_element Targets
    (switch Utilities|FlowControl|Switch|SwitchonEDamageEffectiveness (Class|TypeHelper|GetEffectivenessforMultiplier (.ReturnValue (Class|AbilitySystemComponent|GetGameplayAttributeValue (Class|Battler|GetAbilityComponent _array_element) "(AttributeName=\"TypeMod\",Attribute=/Script/PokemonBattle.TargetDamageStateAttributeSet:TypeMod,AttributeOwner=\"/Script/CoreUObject.Class'/Script/PokemonBattle.TargetDamageStateAttributeSet'\")")))
      (:NotVeryEffective
        (Utilities|Array|Add (LocalVariables|GetNotVeryEffective) (Class|Battler|GetNickname _array_element)))
      (:SuperEffective
        (Utilities|Array|Add (LocalVariables|GetSuperEffective) (Class|Battler|GetNickname _array_element)))))
  (CallFunction|AppendSuperEffectiveMessages Targets (LocalVariables|GetMessageList) (LocalVariables|GetSuperEffective) (LocalVariables|GetNotVeryEffective))
  (return (LocalVariables|GetMessageList)))

(fn AddTypeEffectivenessMessage
  (params (Messages :type Array%20of%20Battle%20Message%20Structures) (Names :type Array%20of%20Texts) (Message :type Text))
  (if (Utilities|Array|IsNotEmpty Names)
    (Utilities|Array|Add Messages (Utilities|Struct|MakeBattleMessage Message 0 "Before"))))

(fn AddNamedTypeEffectivenessMessage
  (params (Messages :type Array%20of%20Battle%20Message%20Structures) (Names :type Array%20of%20Texts) (Format :type Text))
  (if (Utilities|Array|IsNotEmpty Names)
    (Utilities|Array|Add Messages (Utilities|Struct|MakeBattleMessage (Utilities|Text|FormatText Format (Class|StringUtilities|GenerateList Names "and" true)) 0 "Before"))))

(fn AppendSuperEffectiveMessages
  (params (TargetArray :type Array%20of%20Battler%20Interfaces) (Messages :type Array%20of%20Battle%20Message%20Structures) (SuperEffective :type Array%20of%20Texts) (NotVeryEffective :type Array%20of%20Texts))
  (if (> (Utilities|Array|Length TargetArray) 1)
    (CallFunction|AddNamedTypeEffectivenessMessage Messages SuperEffective "It's super effective on {Pkmn}!")
    (CallFunction|AddNamedTypeEffectivenessMessage Messages NotVeryEffective "It's not very effective on {Pkmn}...")
    (else
      (CallFunction|AddTypeEffectivenessMessage Messages SuperEffective "It's super effective!")
      (CallFunction|AddTypeEffectivenessMessage Messages NotVeryEffective "It's not very effective..."))))

(fn GetCriticalHitMessages
  (params (Targets :type Array%20of%20Battler%20Interfaces))
  (for _array_element Targets
    (if (GameplayTags|HasMatchingGameplayTag (Class|Battler|GetAbilityComponent _array_element) "(TagName=\"Battle.MoveTarget.CriticalHit\")")
      (Utilities|Array|Add (LocalVariables|GetCriticalHitNames) (Class|Battler|GetNickname _array_element))))
  (bind _message (CallFunction|AppendCriticalHitMessage Targets (LocalVariables|GetCriticalHitNames)))
  (return _message))

(fn AppendCriticalHitMessage
  (params (TargetArray :type Array%20of%20Battler%20Interfaces) (CriticalHitNames :type Array%20of%20Texts))
  (if (> (Utilities|Array|Length TargetArray) 1)
    (CallFunction|AddNamedTypeEffectivenessMessage (LocalVariables|GetMessageList) CriticalHitNames "A critical hit on {Pkmn}!")
    (else
      (CallFunction|AddTypeEffectivenessMessage (LocalVariables|GetMessageList) CriticalHitNames "A critical hit!")))
  (return (LocalVariables|GetMessageList)))