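; Battle utility function library for a Pokémon-style game, providing burn eligibility, stat-stage checks and localizable battle text.
; CanBurn wraps the generic status-infliction check, while GetStatChangeMessage picks rose or fell wording by sign and magnitude.
; CanRaiseStat and CanLowerStat test stage limits, optionally queuing a message.
; A negative ability-component attribute redirects each to the other, but only CanRaiseStat sets IgnoreInversion, so CanLowerStat bounces back to the minimum check.
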(fn CanBurn
  (params (Ability :type Gameplay%20Ability%20Object%20Reference) (Target :type Battler%20Interface))
  (bind _returnvalue (Class|BattleStatusEffectUtils|CanStatusEffectbeInflicted "BURN" Ability Target "{Pkmn} is already burned!" "It doesn't affect {Pkmn}..."))
  (return _returnvalue))

(fn GetStatChangeMessage
  (params (Battler :type Battler%20Interface) (StatName :type Text) (Change :type Integer))
  (if (> Change 0)
    (bind _message (Battle|Battler|Stats|GetStatRoseMessage Battler StatName Change (LocalVariables|Get__WorldContext)))
    (return _message)
    (elif (< Change 0)
      (bind _message_2 (Battle|Battler|Stats|GetStatFellMessage Battler StatName (* Change -1) (LocalVariables|Get__WorldContext)))
      (return _message_2)
      (else
        (return "")))))

(fn GetStatRoseMessage
  (params (Battler :type Battler%20Interface) (StatName :type Text) (Change :type Integer))
  (switch int Change
    (:Default
      (return (Utilities|Text|FormatText "{Pkmn}'s {Stat} rose drastically!" (Class|Battler|GetNickname Battler) StatName)))
    (:1
      (return (Utilities|Text|FormatText "{Pkmn}'s {Stat} rose!" (Class|Battler|GetNickname Battler) StatName)))
    (:2
      (return (Utilities|Text|FormatText "{Pkmn}'s {Stat} rose sharply!" (Class|Battler|GetNickname Battler) StatName)))))

(fn GetStatFellMessage
  (params (Battler :type Battler%20Interface) (StatName :type Text) (Change :type Integer))
  (switch int Change
    (:Default
      (return (Utilities|Text|FormatText "{Pkmn}'s {Stat} severely fell!" (Class|Battler|GetNickname Battler) StatName)))
    (:1
      (return (Utilities|Text|FormatText "{Pkmn}'s {Stat} fell!" (Class|Battler|GetNickname Battler) StatName)))
    (:2
      (return (Utilities|Text|FormatText "{Pkmn}'s {Stat} harshly fell!" (Class|Battler|GetNickname Battler) StatName)))))

(fn CanRaiseStat
  (params (Battler :type Battler%20Interface) (Stat :type Name) (Messages :type Running%20Message%20Set%20Structure) (ShowMessages :type Boolean) (IgnoreInversion :type Boolean))
  (if (and (< (.ReturnValue (Class|AbilitySystemComponent|GetGameplayAttributeValue (Class|Battler|GetAbilityComponent Battler) "(AttributeName=\"StatStageMultiplier\",Attribute=/Script/PokemonBattle.StatStagesAttributeSet:StatStageMultiplier,AttributeOwner=\"/Script/CoreUObject.Class'/Script/PokemonBattle.StatStagesAttributeSet'\")")) 0.0) (not IgnoreInversion))
    (bind _canlower (Battle|Battler|Stats|CanLowerStat Battler Stat Messages ShowMessages true (LocalVariables|Get__WorldContext)))
    (return _canlower)
    (elif (Class|StatChangeHelpers|StatStageatMax Battler Stat)
      (if ShowMessages
        (Class|BattleSequencer|QueueBattleMessage (Battle|Battler|Stats|GetStatMaxedMessage Battler Stat (LocalVariables|Get__WorldContext))))
      (return false)
      (else
        (return true)))))

(fn CanLowerStat
  (params (Battler :type Battler%20Interface) (Stat :type Name) (Messages :type Running%20Message%20Set%20Structure) (ShowMessages :type Boolean) (IgnoreInversion :type Boolean))
  (if (and (< (.ReturnValue (Class|AbilitySystemComponent|GetGameplayAttributeValue (Class|Battler|GetAbilityComponent Battler) "(AttributeName=\"StatStageMultiplier\",Attribute=/Script/PokemonBattle.StatStagesAttributeSet:StatStageMultiplier,AttributeOwner=\"/Script/CoreUObject.Class'/Script/PokemonBattle.StatStagesAttributeSet'\")")) 0.0) (not IgnoreInversion))
    (bind _canraise (Battle|Battler|Stats|CanRaiseStat Battler Stat Messages ShowMessages false (LocalVariables|Get__WorldContext)))
    (return _canraise)
    (elif (Class|StatChangeHelpers|StatStageatMin Battler Stat)
      (if ShowMessages
        (Class|BattleSequencer|QueueBattleMessage (Battle|Battler|Stats|GetStatMinMessage Battler Stat (LocalVariables|Get__WorldContext))))
      (return false)
      (else
        (return true)))))

(fn GetStatMaxedMessage
  (params (Battler :type Battler%20Interface) (Stat :type Name))
  (return (Utilities|Text|FormatText "{Pkmn}'s {Stat} won't go any higher!" (Class|Battler|GetNickname Battler) (Utilities|Struct|BreakStat (|GetGameData Stat)))))

(fn GetStatMinMessage
  (params (Battler :type Battler%20Interface) (Stat :type Name))
  (return (Utilities|Text|FormatText "{Pkmn}'s {Stat} won't go any lower!" (Class|Battler|GetNickname Battler) (Utilities|Struct|BreakStat (|GetGameData Stat)))))