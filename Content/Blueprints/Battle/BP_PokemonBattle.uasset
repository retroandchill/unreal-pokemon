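; Battle scene actor that presents a Pokémon battle, filling in events for intro, action selection, results and conclusion.
; A timeline swings the pawn on a spring-arm pivot for the wild Pokémon intro, a second returns it, then messages and send-outs lead into battle start.
; Action results recurse through targets, using macros to report hits, crits, effectiveness, fainting and stat changes.
; Victory or loss shows a message and exits the scene.
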(event EventBeginPlay
  (Variables|Battle|Visuals|SetBattlePawnStartingLocation (Transformation|GetActorLocation (Variables|Default|GetBattlePawn)))
  (Variables|Default|SetBattlePawnStartingRotation (Transformation|GetActorRotation (Variables|Default|GetBattlePawn))))

(event EventTick
  (params (DeltaSeconds :type Float%20%28single-precision%29))
  (|CallParentFunction DeltaSeconds))

(event Custom|PlayIntroForWildPokemon
  (Transformation|AttachComponentToComponent (Variables|Default|GetBattlePawn) (Variables|/Game/Blueprints/Battle/WildPokemonIntroPivot.WildPokemonIntroPivot_C|GetSpringArm (Variables|Battle|Visuals|GetWildPokemonIntroPivot)) "None" "SnapToTarget" "SnapToTarget" "KeepRelative" true)
  (bind (_direction _rotation _movement) (Timeline|Timeline PlayFromStart)
    (:Update
      (CallFunction|RotateandMoveIntro _rotation _movement))
    (:Finished
      (CallFunction|ResetPawnAttachment)
      (CallFunction|ResetforBattleStart))))

(event Custom|ResetForBattleStart
  (CallFunction|PreparePawnReturn)
  (bind _lerpfactor (Timeline|Timeline_0 PlayFromStart)
    (:Update
      (CallFunction|LerpPawnReturn _lerpfactor))
    (:Finished
      (Class|PokemonBattle|DisplayBattleIntroMessage))))

(event EventProcessBattleIntroMessage
  (params (Message :type Text%20%28by%20ref%29))
  (|DisplayMessage Message
    (:OnConfirm
      (Class|PokemonBattle|OpponentSendOut))))

(event EventProcessOpponentSendOutMessage
  (params (Message :type Text%20%28by%20ref%29))
  (|DisplayMessage Message
    (:OnConfirm
      (Class|PokemonBattle|OpponentSendOutAnimation))))

(event EventProcessOpponentSendOutAnimation
  (params (OpponentSide :type Battle%20Side%20Interface%20%28by%20ref%29))
  (Class|BattleSide|SendOutBattlers OpponentSide)
  (Class|PokemonBattle|PlayerSendOut))

(event EventPlayBattleIntro
  (CallFunction|PlayIntroforWildPokemon))

(event EventProcessPlayerSendOutMessage
  (params (Message :type Text%20%28by%20ref%29))
  (|DisplayMessage Message
    (:OnConfirm
      (Class|PokemonBattle|PlayerSendOutAnimation))))

(event EventProcessPlayerSendOutAnimation
  (params (PlayerSide :type Battle%20Side%20Interface%20%28by%20ref%29))
  (Class|BattleSide|SendOutBattlers PlayerSide)
  (Class|PokemonBattle|StartBattle))

(event EventBeginActionSelection
  (params (Battler :type Battler%20Interface%20%28by%20ref%29))
  (Class|PokemonBattleScreen|SelectAction (Variables|Default|GetBattleHUD) Battler))

(event Custom|DisplayMessageForResult
  (params (TargetResults :type Array%20of%20Target%20Result%20Structures) (Index :type Integer))
  (bind _output (Utilities|Array|Get(acopy) TargetResults Index))
  (bind _returnvalue (+ Index 1))
  (bind (_target _bhit _damage _secondaryeffects) (Utilities|Struct|BreakTargetResult _output))
  (bind (_damage_2 _effectiveness _bcriticalhit) (Utilities|Struct|BreakBattleDamage _damage))
  (Utilities|HitCheck _bhit)
  (Utilities|CritcalHitCheck _bcriticalhit)
  (Utilities|EffectivenessCheck _target _effectiveness)
  (Utilities|FaintCheck _target
    (:Fainted
      _)
    (:Not%20Fainted
      (Utilities|DisplaySecondaryEffects _target _secondaryeffects)))
  (if (<= (Utilities|Array|Length TargetResults) _returnvalue)
    (Class|PokemonBattle|OnActionResultDisplayFinished)
    (else
      (CallFunction|DisplayMessageforResult TargetResults _returnvalue))))

(event EventDisplayActionResult
  (params (Result :type Action%20Result%20Structure%20%28by%20ref%29))
  (CallFunction|DisplayMessageforResult (.TargetResults (Utilities|Struct|BreakActionResult Result))))

(event EventDisplayAction
  (params (MessageText :type Text%20%28by%20ref%29))
  (|DisplayMessage MessageText
    (:OnConfirm
      (Class|PokemonBattle|ApplyActionResult))))

(event EventProcessPlayerVictory
  (params (IsTrainerBattle :type Boolean))
  (Class|RPGMenusSubsystem|RemoveScreenfromStack)
  (|DisplayMessage "You won!"
    (:OnConfirm
      (Class|PokemonBattle|ExitBattleScene))))

(event EventProcessPlayerLoss
  (params (IsTrainerBattle :type Boolean))
  (Class|RPGMenusSubsystem|RemoveScreenfromStack)
  (|DisplayMessage "You lost!"
    (:OnConfirm
      (Class|PokemonBattle|ExitBattleScene))))

(fn ConstructionScript)

(fn ResetPawnAttachment
  (Transformation|DetachFromActor (Variables|Default|GetBattlePawn) "KeepWorld" "KeepWorld" "KeepRelative")
  (Transformation|AttachActorToActor (Variables|Default|GetBattlePawn) self "None" "KeepRelative" "KeepRelative" "KeepRelative" true))

(fn LerpPawnReturn
  (params (InputPin :type Float%20%28single-precision%29))
  (Transformation|SetActorLocationAndRotation (Variables|Default|GetBattlePawn) (Math|Vector|Lerp(Vector) (Variables|Default|GetCurrentPawnLocation) (Variables|Battle|Visuals|GetBattlePawnStartingLocation) InputPin) (Math|Rotator|Lerp(Rotator) (Variables|Default|GetBattlePawnStartingRotation) (Variables|Default|GetBattlePawnCurrentRotation) InputPin true)))

(fn PreparePawnReturn
  (bind _battlepawn (Variables|Default|GetBattlePawn))
  (Variables|Default|SetCurrentPawnLocation (Transformation|GetActorLocation _battlepawn))
  (Variables|Default|SetBattlePawnCurrentRotation (Transformation|GetActorRotation _battlepawn)))

(fn RotateandMoveIntro
  (params (Yaw :type Float%20%28single-precision%29) (InputPin :type Vector))
  (Transformation|SetActorRotation (Variables|Battle|Visuals|GetWildPokemonIntroPivot) (Math|Rotator|MakeRotator 0.0 -1e+01 Yaw))
  (Transformation|SetActorRelativeLocation (Variables|Battle|Visuals|GetWildPokemonIntroPivot) InputPin))

(fn GetOpponentSidePosition
  (return (Transformation|GetActorTransform (Variables|Battle|Context|GetOpponentTargetPoint))))

(fn GetPlayerSidePosition
  (return (Transformation|GetActorTransform (Variables|Battle|Context|GetPlayerTargetPoint))))

(fn CreateBattleHUD
  (bind _returnvalue (|AddWidgettoStack "/Game/Blueprints/UI/Scenes/PokemonBattleScene.PokemonBattleScene_C"))
  (bind _output_get (Variables|Default|SetBattleHUD _returnvalue))
  (Class|PokemonBattleScreen|SetBattle _output_get self))

(fn RefreshBattleHUD
  (Class|PokemonBattleScreen|Refresh (Variables|Default|GetBattleHUD)))