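; Item utility Blueprint that runs the dialogue and bag changes for giving a Pokémon an item to hold.
; GiveItemtoPokemon rebinds its ItemGiven and ItemNotGiven dispatchers to the caller's callbacks, then branches on the current held item.
; An empty slot takes one item from the bag, while an occupied one prompts for a swap that returns the old item.
; No visible call sets the Pokémon's held item.
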(event EventGiveItemtoPokemon
  (params (WorldContext :type Object%20Object%20Reference) (Item :type Name :default "None") (Pokemon :type Pokemon%20Interface%20%28by%20ref%29) (PokemonIndex :type Integer) (ItemGiven :type Delegate%20%28by%20ref%29) (ItemNotGiven :type Delegate%20%28by%20ref%29))
  (Utilities|FlowControl|Sequence
    (:then_0
      (EventDispatchers|UnbindallEventsfromItemGiven)
      (EventDispatchers|UnbindallEventsfromItemNotGiven))
    (:then_1
      (EventDispatchers|BindEventtoItemGiven ItemGiven))
    (:then_2
      (EventDispatchers|BindEventtoItemNotGiven ItemNotGiven))
    (:then_3
      (bind _helditem (Class|HoldItemUtilities|GetHeldItem Pokemon)
        (:HasItem
          (Utilities|PromptReplaceItem WorldContext Item _helditem Pokemon
            (:ItemGiven
              (Default|CallItemGiven))
            (:ItemNotGiven
              (Default|CallItemNotGiven))))
        (:NoHeldItem
          (Utilities|GiveItem WorldContext Pokemon Item
            (:OnConfirm
              (Default|CallItemGiven))))))))

(fn GetHeldItemPrompt
  (params (Item :type Item%20Structure%20%28by%20ref%29) (Pokemon :type Pokemon%20Interface%20%28by%20ref%29))
  (bind _realportionname (Utilities|Struct|BreakItem Item))
  (return (Utilities|Text|FormatText (select (Class|StringUtilities|StartswithVowelText _realportionname) "{Pkmn} is already holding an {Item}." "{Pkmn} is already holding a {Item}.") _realportionname (Class|Pokemon|GetNickname Pokemon))))