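; Message utility Blueprint that builds the text shown when a Pokémon's status condition is cured.
; GetStatusEffectCuredMessage switches on the status data handle and returns a formatted message with the Pokémon's nickname inserted.
; It has separate wording for sleep, poison, burn, paralysis and freeze.
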(fn GetStatusEffectCuredMessage
  (params (Nickname :type Text) (Status :type Status%20Handle%20Structure))
  (|SwitchonDataHandle Status
    (:SLEEP
      (return (Utilities|Text|FormatText "{Pkmn}  was woken from sleep." Nickname)))
    (:POISON
      (return (Utilities|Text|FormatText "{Pkmn}  was cured of its poisoning." Nickname)))
    (:BURN
      (return (Utilities|Text|FormatText "{Pkmn}'s burn was healed." Nickname)))
    (:PARALYSIS
      (return (Utilities|Text|FormatText "{Pkmn} was cured of paralysis." Nickname)))
    (:FROZEN
      (return (Utilities|Text|FormatText "{Pkmn} was thawed out." Nickname)))))